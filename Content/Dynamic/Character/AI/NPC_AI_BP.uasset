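; AI controller for guard NPCs that sets up a blackboard and runs the guard behavior tree at BeginPlay.
; AI Perception updates feed the blackboard's enemy key, storing a sensed actor and clearing the key when a stimulus is lost.
; Actors tagged "Guard" are ignored, so guards do not register each other as enemies.
; A debug print of pawn, sense and actor names is left unconnected.
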(event `self.ReceiveBeginPlay`
  (bind _blackboardcomponent (`self.UseBlackboard` "/Game/Dynamic/Character/AI/PatrolData.PatrolData"))
  (`self.RunBehaviorTree` "/Game/Dynamic/Character/AI/GuardBehavior.GuardBehavior")
  (set `self.Blackboard Comp` _blackboardcomponent))

(event `self.AIPerception.OnTargetPerceptionUpdated`
  (params (Actor :type "Actor Object Reference") (Stimulus :type "AIStimulus Structure"))
  (`self.Update Blackboard Enemy Key` Stimulus Actor))

(fn `Update Blackboard Enemy Key`
  (params (AIStimulus :type "AIStimulus Structure (by ref)") (Target :type "Actor Object Reference"))
  (bind _blackboard_comp (`self.Blackboard Comp`))
  (bind _enemykey (`self.EnemyKey`))
  (if (`self.ActorHasTag` Target "Guard")
    _
    (elif (`.bSuccessfullySensed` (break `AIStimulus` AIStimulus))
      (`BlackboardComponent.SetValueAsObject` _blackboard_comp _enemykey Target)
      (else
        (`BlackboardComponent.ClearValue` _blackboard_comp _enemykey)))))

(fn `UserConstructionScript`)