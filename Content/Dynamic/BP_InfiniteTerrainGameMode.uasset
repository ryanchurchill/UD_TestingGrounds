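; Game mode for an infinite terrain game that builds the world from chained BP_Tile actors and keeps the score.
; On BeginPlay it spawns a starting run of tiles, each placed at the previous tile's attach location and handed the NavMeshBoundsVolume pool.
; It exposes functions to destroy the oldest tile once the list is two or more over the starting count, and to increment the score when a tile is conquered.
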(event `self.ReceiveBeginPlay`
  (for _ (range (`self.StartingTileCount`))
    (`self.Spawn Tile`)))

(fn `ConditionalDeleteFirstTile`
  (bind _tiles (`self.Tiles`))
  (if (>= (`KismetArrayLibrary.Array_Length` _tiles) (+ (`self.StartingTileCount`) 2))
    (`self.K2_DestroyActor` (`|GetArrayItem` _tiles))
    (`KismetArrayLibrary.Array_Remove` _tiles)))

(fn `GetScore`
  (returns (Score :type Integer))
  (return (`self.Score`)))

(fn `NewTileConquered`
  (`/Engine/EditorBlueprintResources/StandardMacros.IncrementInt` (`self.Score`)))

(fn `Spawn Tile`
  (bind _returnvalue (`|SpawnActorFromClass` "/Game/Dynamic/Terrain/BP_Tile.BP_Tile_C" (`self.NextTileTransform`) "Undefined" "OverrideRootScale" null null))
  (`Tile.SetPool` _returnvalue (`self.NavMeshBoundsVolumePool`))
  (bind _attach_transform (`/Game/Dynamic/Terrain/BP_Tile.Get Attach Location` _returnvalue))
  (set `self.NextTileTransform` _attach_transform)
  (`KismetArrayLibrary.Array_Add` (`self.Tiles`) _returnvalue))

(fn `UserConstructionScript`)