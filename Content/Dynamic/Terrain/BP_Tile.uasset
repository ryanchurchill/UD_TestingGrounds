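; BP_Tile is one segment of an infinite terrain level, which scatters props, rocks and AI characters over itself on BeginPlay.
; Its LockingVolume overlaps, checked against the player, open a green barrier on entry and close it red on exit.
; Exiting also tells BP_InfiniteTerrainGameMode to conditionally delete the first tile, spawn another and record a conquered tile.
; GetAttachLocation exposes the AttachArrow transform.
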(event `self.ReceiveBeginPlay`
  (`self.PlaceActors` "/Game/Dynamic/Terrain/Props/BP_Container.BP_Container_C" 1 3 450.0)
  (`self.PlaceActors` "/Game/Dynamic/Terrain/Props/BP_Box.BP_Box_C" 2 4 100.0)
  (`self.PlaceActors` "/Game/Dynamic/Terrain/Props/BP_Rock01.BP_Rock01_C" 0 4 150.0 1.0 5.0)
  (`self.PlaceActors` "/Game/Dynamic/Terrain/Props/BP_Rock2.BP_Rock2_C" 0 4 250.0 1.0 5.0)
  (`self.PlaceActors` "/Game/Dynamic/Terrain/Props/BP_Rock3.BP_Rock3_C" 0 4 250.0 1.0 5.0)
  (`self.PlaceActors` "/Game/Dynamic/Terrain/Props/BP_Sandbags.BP_Sandbags_C" 1 1 250.0)
  (`self.PlaceAIPawns` "/Game/Dynamic/Character/Behavior/BP_Character.BP_Character_C" 1 3 100.0))

(event `self.Locking Volume.OnComponentBeginOverlap`
  (params (OverlappedComponent :type "PrimitiveComponent Object Reference") (OtherActor :type "Actor Object Reference") (OtherComp :type "PrimitiveComponent Object Reference") (OtherBodyIndex :type Integer) (bFromSweep :type Boolean) (SweepResult :type "HitResult Structure (by ref)"))
  (`self.IsPlayerActor` OtherActor)
  (`self.Unlock`))

(event `self.Locking Volume.OnComponentEndOverlap`
  (params (OverlappedComponent :type "PrimitiveComponent Object Reference") (OtherActor :type "Actor Object Reference") (OtherComp :type "PrimitiveComponent Object Reference") (OtherBodyIndex :type Integer))
  (`self.IsPlayerActor` OtherActor)
  (`self.Lock`)
  (bind _asbp_infinite_terrain_game_mode (cast `/Game/Dynamic/BP_InfiniteTerrainGameMode` (`GameplayStatics.GetGameMode`)))
  (`/Game/Dynamic/BP_InfiniteTerrainGameMode.ConditionalDeleteFirstTile` _asbp_infinite_terrain_game_mode)
  (`/Game/Dynamic/BP_InfiniteTerrainGameMode.Spawn Tile` _asbp_infinite_terrain_game_mode)
  (`/Game/Dynamic/BP_InfiniteTerrainGameMode.NewTileConquered` _asbp_infinite_terrain_game_mode))

(fn `Get Attach Location`
  (returns (`Attach Transform` :type "Transform Structure"))
  (return (`SceneComponent.K2_GetComponentToWorld` (`self.AttachArrow`))))

(fn `Lock`
  (`PrimitiveComponent.SetCollisionEnabled` (`self.Barrier`) "QueryAndPhysics")
  (`PrimitiveComponent.SetMaterial` (`self.Barrier`) 0 "/Game/Dynamic/Terrain/MI_Barrier_Red.MI_Barrier_Red"))

(fn `Unlock`
  (`PrimitiveComponent.SetCollisionEnabled` (`self.Barrier`) "NoCollision")
  (`PrimitiveComponent.SetMaterial` (`self.Barrier`) 0 "/Game/Dynamic/Terrain/MI_Barrier_Green.MI_Barrier_Green"))

(fn `UserConstructionScript`)